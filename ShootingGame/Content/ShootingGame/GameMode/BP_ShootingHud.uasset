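; BP_ShootingHud is the HUD Blueprint for the shooting game mode, owning the on-screen ShootingHudWidget.
; On BeginPlay it creates the widget, stores it in HudWidget and adds it to the viewport.
; Its update functions forward ammo, magazine and HP values to the widget.
; Two more functions pass a world location and visibility to the widget's GuideF indicator.
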(event EventBeginPlay
  (bind _returnvalue (UserInterface|CreateWidget "/Game/ShootingGame/Widget/ShootingHudWidget.ShootingHudWidget_C"))
  (bind _output_get (Variables|Default|SetHudWidget _returnvalue))
  (UserInterface|Viewport|AddtoViewport _output_get 0))

(fn ConstructionScript)

(fn UpdateAmmo
  (params (Ammo :type Integer))
  (Default|SetAmmo (Variables|Default|GetHudWidget) Ammo))

(fn UpdateMag
  (params (Mag :type Integer))
  (Default|SetMag (Variables|Default|GetHudWidget) Mag))

(fn UpdateHp
  (params (CurHp :type Float%20%28single-precision%29) (MaxHp :type Float%20%28single-precision%29))
  (Default|SetHp (Variables|Default|GetHudWidget) CurHp MaxHp))

(fn UpdateGuideF
  (params (WorldLocation :type Vector))
  (Default|SetPositionGuideF (Variables|Default|GetHudWidget) WorldLocation))

(fn SetVisibilityGuideF
  (params (InVisibility :type ESlateVisibility%20Enum :default "Visible"))
  (Default|SetVisibilityGuideF (Variables|Default|GetHudWidget) InVisibility))