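; Player state for the shooting game that holds each player's replicated HP.
; AddDamage subtracts the damage from HP and prints the result for debugging.
; OnRep_Hp logs the new value and, only when the pawn's controller is the first player controller, updates the BP_ShootingHud HP display against a hardcoded maximum.
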(event EventBeginPlay)

(event EventTick
  (params (DeltaSeconds :type Float%20%28single-precision%29)))

(fn ConstructionScript)

(fn AddDamage
  (params (Damage :type Float%20%28single-precision%29))
  (bind _output_get (Variables|Default|SetHp (- (Variables|Default|GetHp) Damage)))
  (Development|PrintString (Utilities|String|Append "Add Damage Result HP = " (Utilities|String|ToString(Float) _output_get)) true true "(R=0.000000,G=0.660000,B=1.000000,A=1.000000)" 6e+01))

(fn OnRepHp
  (bind _returnvalue (Game|GetPlayerController 0))
  ;[1 1 1] (Client)
  (Development|PrintString (Utilities|String|Append "OnRepHP - " (Utilities|String|ToString(Float) (Variables|Default|GetHp))) true true "(R=0.000000,G=0.660000,B=1.000000,A=1.000000)" 6e+01)
  (if (== (Pawn|GetController (Variables|Default|GetPawnPrivate)) _returnvalue)
    (bind _asbp_shooting_hud (Utilities|Casting|CastToBP_ShootingHud (HUD|GetHUD _returnvalue)))
    (Default|UpdateHp _asbp_shooting_hud (Variables|Default|GetHp) 1e+02)))