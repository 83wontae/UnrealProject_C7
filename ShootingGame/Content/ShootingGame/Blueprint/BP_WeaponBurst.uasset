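; BP_WeaponBurst is a burst-fire weapon Blueprint that adds follow-up shots to a trigger pull.
; PullTrigger runs the parent logic, then sets a counter for two additional shots.
; AddShoot plays the rifle single-shot montage on the owning character and decrements the counter, clearing its name-based timer at zero; this file never starts that timer.
; ReleaseTrigger is empty, so releasing does not interrupt the burst.
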(fn ConstructionScript
  (|CallParentFunction))

(fn PullTrigger
  (params (Charactor :type Character%20Object%20Reference))
  (|CallParentFunction Charactor)
  (Variables|Default|SetAddShootCnt 2))

(fn AddShoot
  (bind _owncharacter (Variables|Default|GetOwnCharacter))
  (Utilities|IsValid _owncharacter
    (:Is%20Valid
      (if (> (Variables|Default|GetAddShootCnt) 0)
        (Animation|PlayAnimMontage _owncharacter "/Game/RifleAnimsetPro/Animations/InPlace/Rifle_ShootOnce_Montage.Rifle_ShootOnce_Montage" 1.0 "None")
        (Math|Integer|DecrementInt (Variables|Default|GetAddShootCnt))
        (else
          (Utilities|Time|ClearTimerbyFunctionName 0 "AddShoot"))))))

(fn ReleaseTrigger)