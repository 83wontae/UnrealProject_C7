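; BP_SpawnArea is an item spawn point that keeps a random pickup from its Items list at its location.
; On BeginPlay, SpawnItem runs on the authority only, spawns a random class at the actor's transform and stores it in SpawnedItem.
; It binds to that item's OnDestroyed, and DestroyItem sets a short timer that calls SpawnItem again to respawn a new random item.
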(event EventBeginPlay
  (CallFunction|SpawnItem))

(fn ConstructionScript)

(fn SpawnItem
  (Networking|SwitchHasAuthority
    (:Authority
      (bind _returnvalue (Game|SpawnActorfromClass (.OutItem (Utilities|Array|Random (Variables|Default|GetItems))) (Transformation|GetActorTransform) "Undefined" 0 0))
      (bind _output_get (Variables|Default|SetSpawnedItem _returnvalue))
      (Game|BindEventtoOnDestroyed _output_get (EventDispatchers|CreateEvent :!event DestroyItem)))))

(fn DestroyItem
  (params (DestroyedActor :type Actor%20Object%20Reference))
  (Utilities|Time|SetTimerbyFunctionName 0 "SpawnItem" 3.0))