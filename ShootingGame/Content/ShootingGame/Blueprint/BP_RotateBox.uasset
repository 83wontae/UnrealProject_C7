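; BP_RotateBox is an interactable box whose Cube component starts or stops spinning when a character presses it.
; EventPress calls EnablePlay, which flips the IsPlay flag, while EventRelease does nothing and both return false.
; While IsPlay is set, Tick adds a fixed relative rotation to the Cube each frame without delta-time scaling, so spin speed depends on frame rate.
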(event EventBeginPlay)

(event Collision|EventActorBeginOverlap
  (params (OtherActor :type Actor%20Object%20Reference)))

(event EventTick
  (params (DeltaSeconds :type Float%20%28single-precision%29))
  (if (Variables|Default|GetIsPlay)
    (Transformation|AddRelativeRotation (Variables|Default|GetCube) "0,5.000000, 0" false false)))

(fn ConstructionScript)

(fn EnablePlay
  (Variables|Default|SetIsPlay (not (Variables|Default|GetIsPlay))))

(fn EventPress
  (params (Character :type Character%20Object%20Reference))
  (CallFunction|EnablePlay)
  (return false))

(fn EventRelease
  (params (Character :type Character%20Object%20Reference))
  (return false))