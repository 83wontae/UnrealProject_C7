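; BP_SplineMove is a Blueprint that moves its Cube component back and forth along its Spline.
; On BeginPlay, IsMoveRight selects whether Timeline_0 plays forward or in reverse.
; Each update scales the timeline value by spline length and sets the cube's world location and rotation from that distance.
; When the timeline finishes, it flips IsMoveRight and repeats the branch, creating a continuous ping-pong loop.
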(event EventBeginPlay
  (bind _spline (Variables|Default|GetSpline))
  (if (Variables|Default|GetIsMoveRight) :!label _label
    (bind _value (Timeline|Timeline_0 Play)
      (:Update
        (Transformation|SetWorldLocationAndRotation (Variables|Default|GetCube) (Spline|GetLocationatDistanceAlongSpline _spline (* (Spline|GetSplineLength (Variables|Default|GetSpline)) _value) "World") (Spline|GetRotationatDistanceAlongSpline _spline (* (Spline|GetSplineLength (Variables|Default|GetSpline)) _value) "World") false false))
      (:Finished
        (Variables|Default|SetIsMoveRight (not (Variables|Default|GetIsMoveRight)))
        (goto _label)))
    (else
      (Timeline|Timeline_0 Reverse))))

(fn ConstructionScript)