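; Lobby game mode for the shooting game that hosts a dedicated-server session and moves players into the match map.
; BeginPlay creates an Advanced Sessions session with a hardcoded server name and prints success or failure.
; PostLogin and HandleStartingNewPlayer print debug messages for each joiner.
; Once at least two players are present, HandleStartingNewPlayer runs a servertravel console command to ThirdPersonExampleMap.
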(event EventBeginPlay
  (|AdvancedSession (Utilities|Array|MakeArray (Class|AdvancedSessionsLibrary|MakeLiteralSessionPropertyString "ServerName" "wontae")) (Game|GetPlayerController 0) 100 0 false true true false true true false false false true
    (:OnSuccess
      (Development|PrintString "세션 생성 성공"))
    (:OnFailure
      (Development|PrintString "세션 생성 실패"))))

(event EventHandleStartingNewPlayer
  (params (NewPlayer :type Player%20Controller%20Object%20Reference))
  (|CallParentFunction NewPlayer)
  (Development|PrintString (Utilities|String|Append "Handel Starting NewPlayer - " (Utilities|GetDisplayName NewPlayer)) true true "(R=0.000000,G=0.660000,B=1.000000,A=1.000000)" 6e+01)
  (bind _returnvalue (Class|GameModeBase|GetNumPlayers))
  (Development|PrintString (Utilities|String|Append "NumPlayers - " (Utilities|String|ToString(Integer) _returnvalue)))
  (if (>= _returnvalue 2)
    (Development|ExecuteConsoleCommand "servertravel ThirdPersonExampleMap" 0)))

(event EventPostLogin
  (params (NewPlayer :type Player%20Controller%20Object%20Reference))
  (|CallParentFunction NewPlayer)
  (Development|PrintString (Utilities|String|Append "OnPostLogin NewPlayer - " (Utilities|GetDisplayName NewPlayer)) true true "(R=0.000000,G=0.660000,B=1.000000,A=1.000000)" 6e+01))

(fn ConstructionScript)